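; BP_NPC_SmallKnight is an NPC that advances the Find Small Knight quest when the player's paper character first overlaps it.
; A DoOnce gate limits this to one trigger, then the NPC looks up the BP_Quest_FindSmallKnight actor in the level.
; It updates that quest's first current objective by one, marks the quest inactive, and prints a message if the quest is complete.
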(event `self.ReceiveActorBeginOverlap`
  (params (OtherActor :type "Actor Object Reference"))
  (cast `/Game/TDCharacter/Blueprints/BP_PaperCharacter` OtherActor)
  (`/Engine/EditorBlueprintResources/StandardMacros.DoOnce` false
    (:`Completed`
      (bind _returnvalue (`GameplayStatics.GetActorOfClass` "/Game/QuestSystem/FindAKnight/BP_Quest_FindSmallKnight.BP_Quest_FindSmallKnight_C"))
      (`/Engine/EditorBlueprintResources/StandardMacros.IsValid` _returnvalue
        (:`Is Valid`
          (bind _output_get (set `self.Objective` (`|GetArrayItem` (`Quest.CurrentObjectives` _returnvalue))))
          (`/Engine/EditorBlueprintResources/StandardMacros.IsValid` _output_get
            (:`Is Valid`
              (`Objective.Update` _output_get 1)
              (set `Quest.bIsActive` false _returnvalue)
              (if (`Quest.IsQuestComplete` _returnvalue)
                (`KismetSystemLibrary.PrintString` "Quest completed!")))))))))

(fn `UserConstructionScript`)