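; BP_NPC is a quest-giver NPC that turns in the FindSmallKnight quest and hands out the ClearACave quest.
; Player overlap advances the first objective, then on completion destroys the quest and objectives and binds the dialog UI's third button.
; Clicking that button runs an EQS spawn-location query, which spawns ten minions per returned location with debug spheres, plus the new quest actor.
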(event `self.ReceiveActorBeginOverlap`
  (params (OtherActor :type "Actor Object Reference"))
  (cast `/Game/TDCharacter/Blueprints/BP_Character` OtherActor)
  (`|ExecutionSequence`
    (:`then_0`
      (`/Engine/EditorBlueprintResources/StandardMacros.DoOnce` false :!label _label
        (:`Completed`
          (bind _outactors (`GameplayStatics.GetAllActorsOfClass` "/Game/QuestSystem/BP_Quest_FindSmallKnight.BP_Quest_FindSmallKnight_C"))
          (bind _output (`|GetArrayItem` _outactors))
          (`/Engine/EditorBlueprintResources/StandardMacros.IsValid` _output
            (:`Is Valid`
              (bind _currentobjectives (`Quest.CurrentObjectives` _output))
              (bind _output_get (set `self.CurrentObjectives` _currentobjectives))
              (bind _output_get_2 (set `self.Objective` (`|GetArrayItem` _currentobjectives)))
              (`/Engine/EditorBlueprintResources/StandardMacros.IsValid` _output_get_2
                (:`Is Valid`
                  (`Objective.Update` _output_get_2 1)
                  (if (`Quest.IsQuestComplete` _output)
                    (`KismetSystemLibrary.PrintString` "Quest completed!")
                    (`self.K2_DestroyActor` _output)
                    (`|ExecutionSequence`
                      (:`then_0`
                        (`/Engine/EditorBlueprintResources/StandardMacros.IsValid` (`|GetArrayItem` _output_get 8)
                          (:`Is Valid`
                            (for _array_element _output_get
                              (`self.K2_DestroyActor` _array_element)))))
                      (:`then_1`
                        (`/Engine/EditorBlueprintResources/StandardMacros.IsValid` _output_get_2
                          (:`Is Valid`
                            (`self.K2_DestroyActor` _output_get_2)
                            (bind _foundwidgets (`WidgetBlueprintLibrary.GetAllWidgetsOfClass` "/Game/DialogSystem/Widget/BP_DialogUI.BP_DialogUI_C" false))
                            (bind _output_get_3 (set `self.WidgetDialog` (`|GetArrayItem` _foundwidgets)))
                            (add `Button.OnClicked` (`/Game/DialogSystem/Widget/BP_DialogUI.Button_3` _output_get_3) (delegate `OnClicked_Event_0`))))))))))))))))

(event `OnClicked_Event_0`
  (`/Engine/EditorBlueprintResources/StandardMacros.DoOnce` false
    (:`Completed`
      (bind _returnvalue (`EnvQueryManager.RunEQSQuery` "/Game/BluePrints/Foes/EQuery_FindSpawnLocation.EQuery_FindSpawnLocation" self "RandomBest25Pct"))
      (add `EnvQueryInstanceBlueprintWrapper.OnQueryFinishedEvent` _returnvalue (delegate `OnQueryFinishedEvent_Event_0`)))))

(event `self.ReceiveBeginPlay`)

(event `OnQueryFinishedEvent_Event_0`
  (params (QueryInstance :type "EnvQueryInstanceBlueprintWrapper Object Reference") (QueryStatus :type "EEnvQueryStatus Enum" :default "Processing"))
  (switch `EEnvQueryStatus` QueryStatus
    (:`Success`
      (bind _resultlocations (`EnvQueryInstanceBlueprintWrapper.GetQueryResultsAsLocations` QueryInstance))
      (for _array_element _resultlocations
        (`KismetSystemLibrary.DrawDebugSphere` _array_element 20.0 12 (struct :`R` 0.089069 :`G` 1.0 :`A` 1.0) 2.0 2.0)
        (for _ (range 10)
          (`AIBlueprintHelperLibrary.SpawnAIFromClass` "/Game/BluePrints/Foes/BP_Minion.BP_Minion_C" null _array_element))
        (`|SpawnActorFromClass` "/Game/QuestSystem/BP_Quest_ClearACave.BP_Quest_ClearACave_C" (`KismetMathLibrary.Conv_VectorToTransform` (`self.K2_GetActorLocation` self)) "AdjustIfPossibleButAlwaysSpawn" "OverrideRootScale" null self)
        (set `self.Quest` null)
        (`KismetSystemLibrary.PrintString` "Quest Accepted!" true false (struct :`R` 1.0 :`G` 0.088168 :`A` 1.0) 3.0)
        (goto _label :!via `Reset`)))))

(fn `UserConstructionScript`)