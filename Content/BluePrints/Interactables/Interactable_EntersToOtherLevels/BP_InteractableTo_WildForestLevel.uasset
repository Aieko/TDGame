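; Interactable level entrance that sends the player to the Wild Forest level when used.
; OnUse casts to the paper character, its journal UI and the game instance, stopping if any cast fails.
; An IsAllSaved-gated while loop copies Health and Gold into the game instance, clearing the flag, before the level opens.
; The journal's CurrentQuests is read by an unused node, so quests are not saved here.
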(event `self.OnUse`
  (params (Character :type "TDPaperCharacter Object Reference"))
  (bind _asbp_paper_character (cast `/Game/TDCharacter/Blueprints/BP_PaperCharacter` Character))
  (bind _asbp_journal_main (cast `/Game/Journal/Widget/BP_JournalMain` (`TDPaperCharacter.UIJournal` _asbp_paper_character)))
  (bind _astdgame_instance (cast `/Game/TDCharacter/Blueprints/TDGameInstance` (`GameplayStatics.GetGameInstance`)))
  (while (`self.IsAllSaved`)
    (set `/Game/TDCharacter/Blueprints/TDGameInstance.Health` (`TDHealthComponent.Health` (`TDPaperCharacter.HealthComp` _asbp_paper_character)) _astdgame_instance)
    (set `/Game/TDCharacter/Blueprints/TDGameInstance.Gold` (`TDInventoryComponent.Gold` (`/Game/TDCharacter/Blueprints/BP_PaperCharacter.InventoryComponent` _asbp_paper_character)) _astdgame_instance)
    (set `self.IsAllSaved` false))
  (`GameplayStatics.OpenLevelBySoftObjectPtr` "/Game/Maps/Level2_WildForest.Level2_WildForest"))

(fn `UserConstructionScript`)