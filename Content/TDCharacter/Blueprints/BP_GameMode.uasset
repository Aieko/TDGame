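; BP_GameMode is a game mode Blueprint that starts the find-small-knight quest when play begins.
; After a short delay, it spawns BP_Quest_FindSmallKnight at the player character's location, with that character as instigator.
; It stores the spawned actor as the current quest and its first objective as the current objective, then prints a prompt if that objective is valid.
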(event `self.ReceiveBeginPlay`
  (bind _returnvalue (`GameplayStatics.GetPlayerCharacter` 0))
  (`KismetSystemLibrary.Delay` 0.2)
  (bind _returnvalue_2 (`|SpawnActorFromClass` "/Game/QuestSystem/BP_Quest_FindSmallKnight.BP_Quest_FindSmallKnight_C" (`KismetMathLibrary.Conv_VectorToTransform` (`self.K2_GetActorLocation` _returnvalue)) "AlwaysSpawn" "OverrideRootScale" null _returnvalue))
  (bind _output_get (set `self.CurrentQuest_CPP` _returnvalue_2))
  (bind _output (`|GetArrayItem` (`Quest.CurrentObjectives` _output_get)))
  (set `self.CurrentObjective` _output)
  (`/Engine/EditorBlueprintResources/StandardMacros.IsValid` _output
    (:`Is Valid`
      (`KismetSystemLibrary.PrintString` "Find a Knight!" true false (struct :`G` 0.66 :`B` 1.0 :`A` 1.0) 15.0))))

(fn `UserConstructionScript`)