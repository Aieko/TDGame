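; Paper character Blueprint for the player that manages the inventory, dialogue and quest journal UI.
; Inventory and journal toggles switch cursor and input mode; the journal widget is created once at BeginPlay, the inventory on each opening.
; Dialogue finds the associated NPC's row by name in DT_DialogueList and opens a dialogue widget with it.
; Debug prints report inventory items at start and, on G, the game instance's quest objectives.
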(event `self.ReceiveBeginPlay`
  ;[1 1 1] OnBeginPlay
  (`|ExecutionSequence`
    (:`then_0`
      (for _array_element (`TDInventoryComponent.Items` (`self.InventoryComponent`))
        (`/Engine/EditorBlueprintResources/StandardMacros.IsValid` _array_element
          (:`Is Valid`
            (`KismetSystemLibrary.PrintString` "Hello from Character Inventory" true true (struct :`R` 1.0 :`G` 0.211545 :`A` 1.0) 5.0)))))
    (:`then_1`
      (bind _returnvalue (`|CreateWidget` "/Game/Journal/Widget/BP_JournalMain.BP_JournalMain_C" (`GameplayStatics.GetPlayerController` 0)))
      (set `self.UIJournal` _returnvalue))))

(event `self.ToggleInventoryUI`
  (bind _returnvalue (`GameplayStatics.GetPlayerController` 0))
  (bind _returnvalue_2 (`GameplayStatics.GetPlayerController` 0))
  ;[1 1 1] InventoryToggle
  (if (`self.bIsInventoryOpen`)
    (`Widget.RemoveFromParent` (`self.InventoryRef`))
    (set `PlayerController.bShowMouseCursor` false _returnvalue)
    (`WidgetBlueprintLibrary.SetInputMode_GameOnly` _returnvalue)
    (set `self.bIsInventoryOpen` false)
    (else
      (bind _returnvalue_3 (`|CreateWidget` "/Game/InventorySystem/Widgets/WBP_Inventory.WBP_Inventory_C" (`GameplayStatics.GetPlayerController` 0)))
      (bind _output_get (set `self.InventoryRef` _returnvalue_3))
      (`UserWidget.AddToViewport` _output_get 0)
      (set `PlayerController.bShowMouseCursor` true _returnvalue_2)
      (`WidgetBlueprintLibrary.SetInputMode_GameAndUIEx` _returnvalue_2 _returnvalue_3)
      (set `self.bIsInventoryOpen` true))))

(event `self.ToggleDialogueUI`
  (bind _associatedpawn (`self.AssociatedPawn`))
  ;[1 1 1] DialoguesToggle
  (if (not (`self.bIsTalking`))
    (bind _outrownames (`DataTableFunctionLibrary.GetDataTableRowNames` "/Game/DialogSystem/DataTable/DT_DialogueList.DT_DialogueList"))
    (for _array_element _outrownames
      (bind _returnvalue (`|GetDataTableRow` "/Game/DialogSystem/DataTable/DT_DialogueList.DT_DialogueList" _array_element)
        (:`then`
          (bind (_npc_name _dialogue) (break `/Game/DialogSystem/DataTable/DialogueStuct` _returnvalue))
          (if (`KismetTextLibrary.EqualEqual_TextText` _npc_name (`TDIdleNPC.NPCName` _associatedpawn))
            (bind _returnvalue_2 (`|CreateWidget` "/DialoguePlugin/UI/DemoDialogueWidget.DemoDialogueWidget_C" (`GameplayStatics.GetPlayerController` 0) _dialogue _associatedpawn))
            (`UserWidget.AddToViewport` _returnvalue_2 0)
            (set `self.bIsTalking` true)))))))

(event `self.ToggleJournalUI`
  (bind _returnvalue (`GameplayStatics.GetPlayerController` 0))
  (bind _returnvalue_2 (`GameplayStatics.GetPlayerController` 0))
  (bind _uijournal (`self.UIJournal`))
  ;[1 1 1] JournalToggle
  (`/Engine/EditorBlueprintResources/StandardMacros.IsValid` _uijournal
    (:`Is Valid`
      (if (`Widget.IsInViewport` _uijournal)
        (`WidgetBlueprintLibrary.SetInputMode_GameOnly` _returnvalue_2)
        (set `PlayerController.bShowMouseCursor` false _returnvalue_2)
        (`Widget.RemoveFromParent` (`self.UIJournal`))
        (else
          (`UIJournal.Show` (`self.UIJournal`))
          (set `PlayerController.bShowMouseCursor` true _returnvalue)
          (`WidgetBlueprintLibrary.SetInputMode_GameAndUIEx` _returnvalue (`self.UIJournal`)))))))

(event `Key|G`
  (params (Key :type "Key Structure"))
  (:`Pressed`
    (bind _astdgame_instance (cast `/Game/TDCharacter/Blueprints/TDGameInstance` (`GameplayStatics.GetGameInstance`)))
    (for (_array_element _array_index) (`/Game/TDCharacter/Blueprints/TDGameInstance.AvaliableQuestes` _astdgame_instance)
      (`/Engine/EditorBlueprintResources/StandardMacros.IsValid` _array_element
        (:`Is Valid`
          (bind _output (`|GetArrayItem` (`Quest.CurrentObjectives` _array_element)))
          (`/Engine/EditorBlueprintResources/StandardMacros.IsValid` _output
            (:`Is Valid`
              (`KismetSystemLibrary.PrintString` (`KismetSystemLibrary.GetDisplayName` _output) true true (struct :`R` 1.0 :`G` 0.063102 :`A` 1.0))
              (`KismetSystemLibrary.PrintString` (`KismetStringLibrary.Conv_IntToString` _array_index) true true (struct :`R` 1.0 :`G` 0.063102 :`A` 1.0)))))))))

(fn `UserConstructionScript`)