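; BP_Character is a character Blueprint that opens and closes a dialogue UI for the local player.
; On BeginPlay it creates a BP_DialogUI widget and keeps a reference to it.
; ToggleUI passes the character's Questions to the widget and shows it with cursor and UI-focused input, or clears subtitles, removes it and restores game-only input.
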(event `self.ReceiveBeginPlay`
  (bind _returnvalue (`|CreateWidget` "/Game/DialogSystem/Widget/BP_DialogUI.BP_DialogUI_C" (`GameplayStatics.GetPlayerController` 0)))
  (set `self.UI` _returnvalue))

(event `self.ToggleUI`
  (bind _returnvalue (`GameplayStatics.GetPlayerController` 0))
  (bind _ui (`self.UI`))
  (bind _ui_2 (`self.UI`))
  (`/Engine/EditorBlueprintResources/StandardMacros.IsValid` _ui_2
    (:`Is Valid`
      (if (`Widget.IsInViewport` _ui_2)
        (`WidgetBlueprintLibrary.SetInputMode_GameOnly` (`GameplayStatics.GetPlayerController` 0))
        (set `PlayerController.bShowMouseCursor` false (`GameplayStatics.GetPlayerController` 0))
        (`DIalogUI.UpdateSubtitles` _ui (`self.ClearSubtitles`))
        (`Widget.RemoveFromParent` _ui)
        (else
          (set `DIalogUI.Questions` (`self.Questions`) _ui_2)
          (`DIalogUI.Show` _ui_2)
          (set `PlayerController.bShowMouseCursor` true _returnvalue)
          (`WidgetBlueprintLibrary.SetInputMode_GameAndUIEx` _returnvalue _ui))))))

(fn `UserConstructionScript`)